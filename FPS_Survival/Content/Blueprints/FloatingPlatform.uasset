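; Floating platform actor that snaps from a start transform to an end transform when gravity is switched off.
; BeginPlay clears GravityOff, stores the Platform's transform origin as StartPos and sets EndPos to an empty value.
; Pressing the 4 key sets GravityOff, with no way to switch it back.
; Tick sets the actor transform to StartPos or EndPos from that flag every frame, without sweep or interpolation.
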(event EventBeginPlay
  (Variables|Default|SetGravityOff false)
  (bind _returnvalue (Class|MovieSceneTransformOrigin|GetTransformOrigin(Message) (Variables|Default|GetPlatform)))
  (Variables|Default|SetStartPos _returnvalue)
  (Variables|Default|SetEndPos ""))

(event Collision|EventActorBeginOverlap
  (params (OtherActor :type Actor%20Object%20Reference)))

(event EventTick
  (params (DeltaSeconds :type Float%20%28single-precision%29))
  (Utilities|FlowControl|Sequence
    (:then_0
      (if (Variables|Default|GetGravityOff)
        (Transformation|SetActorTransform (Variables|Default|GetEndPos))
        (else
          (Transformation|SetActorTransform (Variables|Default|GetStartPos)))))))

(event Input|KeyboardEvents|4
  (params (Key :type Key%20Structure :default "None"))
  (:Pressed
    (Variables|Default|SetGravityOff true)))

(fn ConstructionScript)